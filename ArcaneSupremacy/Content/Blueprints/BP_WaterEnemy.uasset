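; BP_WaterEnemy is a water-element enemy that takes typed damage and dies when its health runs out.
; ApplyDamage doubles Earth damage, halves Fire damage and passes other types through unchanged before subtracting it from Health.
; At zero health or below it detaches from its controller, waits briefly and destroys itself.
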(event EventApplyDamage
  (params (Damage :type Float%20%28single-precision%29) (AttackType :type String))
  (Variables|Default|SetDamageTaken Damage)
  (bind _output_get (Variables|Default|SetAttackingType AttackType))
  (if (Utilities|Enum|Equal(Enum) _output_get "Earth")
    (bind _output_get_2 (Variables|Default|SetDamageTaken (* (Variables|Default|GetDamageTaken) 2.0)))
    (Variables|Default|SetHealth (- (Variables|Default|GetHealth) _output_get_2))
    (elif (Utilities|Enum|Equal(Enum) (Variables|Default|GetAttackingType) "Fire")
      (Variables|Default|SetDamageTaken (* (Variables|Default|GetDamageTaken) 0.5))
      (Variables|Default|SetHealth (- (Variables|Default|GetHealth) (Variables|Default|GetDamageTaken)))
      (else
        (Variables|Default|SetHealth (- (Variables|Default|GetHealth) (Variables|Default|GetDamageTaken))))))
  (if (<= (Variables|Default|GetHealth) 0.0)
    (Class|Pawn|DetachfromControllerPendingDestroy)
    (Utilities|FlowControl|Delay 2.0)
    (Actor|DestroyActor)))

(fn ConstructionScript)