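; BP_Enemy is an enemy actor that takes elemental damage and dies when its health runs out.
; A custom event receives a damage amount and attack type, doubles Earth damage, halves Fire damage, and subtracts the result from Health.
; When Health reaches zero or below, it waits briefly and then destroys itself.
; BeginPlay, overlap and Tick are unused stubs.
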(event Custom|CustomEvent
  (params (Damage :type Float%20%28single-precision%29) (AttackType :type String))
  (Variables|Default|SetDamageTaken Damage)
  (bind _output_get (Variables|Default|SetAttackingType AttackType))
  (if (Utilities|Enum|Equal(Enum) _output_get "Earth")
    (bind _output_get_2 (Variables|Default|SetDamageTaken (* (Variables|Default|GetDamageTaken) 2.0)))
    (Variables|Default|SetHealth (- (Variables|Default|GetHealth) _output_get_2))
    (elif (Utilities|Enum|Equal(Enum) (Variables|Default|GetAttackingType) "Fire")
      (Variables|Default|SetDamageTaken (* (Variables|Default|GetDamageTaken) 0.5))
      (Variables|Default|SetHealth (- (Variables|Default|GetHealth) (Variables|Default|GetDamageTaken)))
      (else
        (Variables|Default|SetHealth (- (Variables|Default|GetHealth) (Variables|Default|GetDamageTaken))))))
  (if (<= (Variables|Default|GetHealth) 0.0)
    (Utilities|FlowControl|Delay 2.0)
    (Actor|DestroyActor)))

(event EventBeginPlay
  (|CallParentFunction) ; This node is disabled and will not be called.\nDrag off pins to build functionality.
)

(event EventTick
  (params (DeltaSeconds :type Float%20%28single-precision%29))
  (|CallParentFunction DeltaSeconds) ; This node is disabled and will not be called.\nDrag off pins to build functionality.
)

(event Collision|EventActorBeginOverlap
  (params (OtherActor :type Actor%20Object%20Reference))
  (|CallParentFunction OtherActor) ; This node is disabled and will not be called.\nDrag off pins to build functionality.
)

(fn ConstructionScript)