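; BP_TurnBased tracks whose turn it is in a turn-based system through a TurnCount index over the active characters.
; NextTurn increments the index without bounds checking.
; Tick runs CheckTurnOutOfBounds every frame, wrapping TurnCount to zero at NumActiveCharacters or to the last index when it drops below zero.
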(event Custom|CheckTurnOutOfBounds
  (if (>= (Variables|Default|GetturnCount) (Variables|Default|GetnumActiveCharacters))
    (Variables|Default|SetturnCount 0)
    (elif (<= (Variables|Default|GetturnCount) -1)
      (Variables|Default|SetturnCount (- (Variables|Default|GetnumActiveCharacters) 1)))))

(event EventTick
  (params (DeltaSeconds :type Float%20%28single-precision%29))
  (CallFunction|CheckTurnOutOfBounds))

(fn ConstructionScript)

(fn NextTurn
  (Variables|Default|SetturnCount (+ (Variables|Default|GetturnCount) 1)))