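; BP_Projectile is an elemental attack projectile that damages non-player actors it overlaps.
; Half a second after BeginPlay, it swaps the Sphere material to a fire, water or earth storm look based on AttackType.
; On overlap with an actor implementing IDamageable and lacking the Player tag, it sends Damage and AttackType through the interface, then destroys itself.
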(event EventBeginPlay
  (bind _sphere (Variables|Default|GetSphere))
  (Utilities|FlowControl|Delay 0.5)
  (if (Utilities|Enum|Equal(Enum) (Variables|Default|GetAttackType) "Fire")
    (Rendering|Material|SetMaterial _sphere 0 "/Game/FXVarietyPack/Materials/MI_ky_storm01_fire.MI_ky_storm01_fire")
    (elif (Utilities|Enum|Equal(Enum) (Variables|Default|GetAttackType) "Water")
      (Rendering|Material|SetMaterial _sphere 0 "/Game/FXVarietyPack/Materials/MI_ky_storm01_aqua.MI_ky_storm01_aqua")
      (elif (Utilities|Enum|Equal(Enum) (Variables|Default|GetAttackType) "Earth")
        (Rendering|Material|SetMaterial _sphere 0 "/Game/FXVarietyPack/Materials/M_ky_storm01.M_ky_storm01")))))

(event Collision|EventActorBeginOverlap
  (params (OtherActor :type Actor%20Object%20Reference))
  (if (Utilities|DoesObjectImplementInterface OtherActor "/Game/Blueprints/IDamageable.IDamageable_C")
    (if (not (Actor|ActorHasTag OtherActor "Player"))
      (Class|IDamageable|ApplyDamage(Message) OtherActor (Variables|Default|GetDamage) (Variables|Default|GetAttackType))
      (Actor|DestroyActor))))

(fn ConstructionScript)