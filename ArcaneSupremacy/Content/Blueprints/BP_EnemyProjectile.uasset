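; BP_EnemyProjectile is an elemental enemy projectile that damages the player on impact.
; Shortly after BeginPlay it picks the sphere's storm material from its AttackType of Fire, Water or Earth.
; On hit, if the other actor implements IDamageable and has the Player tag, it sends Damage and AttackType through the interface message, then destroys itself.
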(event EventBeginPlay
  (bind _sphere (Variables|Default|GetSphere))
  (Utilities|FlowControl|Delay 0.01)
  (if (Utilities|Enum|Equal(Enum) (Variables|Default|GetAttackType) "Fire")
    (Rendering|Material|SetMaterial _sphere 0 "/Game/FXVarietyPack/Materials/MI_ky_storm01_fire.MI_ky_storm01_fire")
    (elif (Utilities|Enum|Equal(Enum) (Variables|Default|GetAttackType) "Water")
      (Rendering|Material|SetMaterial _sphere 0 "/Game/FXVarietyPack/Materials/MI_ky_storm01_aqua.MI_ky_storm01_aqua")
      (elif (Utilities|Enum|Equal(Enum) (Variables|Default|GetAttackType) "Earth")
        (Rendering|Material|SetMaterial _sphere 0 "/Game/FXVarietyPack/Materials/M_ky_storm01.M_ky_storm01")))))

(event Collision|EventHit
  (params (MyComp :type Primitive%20Component%20Object%20Reference) (Other :type Actor%20Object%20Reference) (OtherComp :type Primitive%20Component%20Object%20Reference) (bSelfMoved :type Boolean) (HitLocation :type Vector :default "0, 0, 0") (HitNormal :type Vector :default "0, 0, 0") (NormalImpulse :type Vector :default "0, 0, 0") (Hit :type Hit%20Result%20Structure%20%28by%20ref%29))
  (if (and (Utilities|DoesObjectImplementInterface Other "/Game/Blueprints/IDamageable.IDamageable_C") (Actor|ActorHasTag Other "Player"))
    (Class|IDamageable|ApplyDamage(Message) Other (Variables|Default|GetDamage) (Variables|Default|GetAttackType))
    (Actor|DestroyActor)))

(fn ConstructionScript)