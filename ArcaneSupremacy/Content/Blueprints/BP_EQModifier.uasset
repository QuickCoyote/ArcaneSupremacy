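; BP_EQModifier plays a song and samples its frequency spectrum over time to supply values for an audio-reactive, equalizer-style effect.
; Tick refreshes the Frequencies array with CalculateFrequencySpectrum, using game time offset slightly backward as the sample position.
; GetFrequencyValue runs its own analysis over a longer window and returns a clamped-index band, independent of the stored array.
; ScaleBars converts an input value into a bar scale using a clamped cubic curve with a small minimum.
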(event EventTick
  (params (DeltaSeconds :type Float%20%28single-precision%29))
  (bind _outspectrum (Class|SoundVisualizationStatics|CalculateFrequencySpectrum (Variables|Default|GetSong) 0 (+ (Utilities|Time|GetGameTimeinSeconds) -0.3) 0.1 (Variables|Default|GetSpectrum%20Width)))
  (Variables|Default|SetFrequencies _outspectrum))

(event EventBeginPlay
  (bind _audio (Variables|Default|GetAudio))
  (Audio|Components|Audio|SetSound _audio (Variables|Default|GetSong))
  (Audio|Components|Audio|Play _audio -2.0))

(fn ConstructionScript)

(fn ScaleBars
  (params (A :type Float%20%28single-precision%29))
  (bind _returnvalue (/ A 15.0))
  (bind _returnvalue_2 (Math|Float|Clamp(Float) _returnvalue 0.0 2.75))
  (return (+ (* _returnvalue_2 _returnvalue_2 _returnvalue_2) 0.1)))

(fn GetFrequencyValue
  (params (Frequency :type Integer))
  (bind _outspectrum (Class|SoundVisualizationStatics|CalculateFrequencySpectrum (Variables|Default|GetSong) 0 (+ (Utilities|Time|GetGameTimeinSeconds) -0.3) 0.17 (Variables|Default|GetSpectrum%20Width)))
  (return (Utilities|Array|Get(acopy) _outspectrum (Math|Integer|Clamp(Integer) Frequency 0 (Variables|Default|GetSpectrum%20Width)))))