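; BP_EnemyProjectileFire is a homing enemy projectile that damages IDamageable actors on hit and then destroys itself.
; Each Tick sets a player character mesh as homing target and resets velocity to a fixed X vector.
; An overlapping player who is blocking destroys it.
; FindPlayerTarget tracks the closest character but returns the loop's current element instead of ClosestTarget.
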(event EventBeginPlay
  (Utilities|FlowControl|Delay 0.01)
  (Components|DestroyComponent (Variables|Default|GetBPC_MusicModifier)))

(event EventTick
  (params (DeltaSeconds :type Float%20%28single-precision%29))
  (bind _projectilemovement (Variables|Default|GetProjectileMovement))
  (if (and (Variables|/Game/ThirdPersonBP/Blueprints/ThirdPersonCharacter.ThirdPersonCharacter_C|Getblocking (Variables|Default|GetPlayer)) (Variables|Default|GetBlockable))
    (Actor|DestroyActor)
    (else
      (bind _enemytarget (CallFunction|FindPlayerTarget))
      (Variables|/Script/Engine.ProjectileMovementComponent|SetHomingTargetComponent _projectilemovement _enemytarget)
      (Variables|/Script/Engine.ProjectileMovementComponent|SetbIsHomingProjectile _projectilemovement true)
      (Variables|/Script/Engine.MovementComponent|SetVelocity _projectilemovement "1000.000000, 0, 0"))))

(event Collision|EventHit
  (params (MyComp :type Primitive%20Component%20Object%20Reference) (Other :type Actor%20Object%20Reference) (OtherComp :type Primitive%20Component%20Object%20Reference) (bSelfMoved :type Boolean) (HitLocation :type Vector :default "0, 0, 0") (HitNormal :type Vector :default "0, 0, 0") (NormalImpulse :type Vector :default "0, 0, 0") (Hit :type Hit%20Result%20Structure%20%28by%20ref%29))
  (if (Utilities|DoesObjectImplementInterface Other "/Game/Blueprints/IDamageable.IDamageable_C")
    (Class|IDamageable|ApplyDamage(Message) Other (Variables|Default|GetDamage) (Variables|Default|GetAttackType))
    (Actor|DestroyActor)))

(event Collision|EventActorBeginOverlap
  (params (OtherActor :type Actor%20Object%20Reference))
  (bind _asthird_person_character (Utilities|Casting|CastToThirdPersonCharacter OtherActor))
  (Variables|Default|SetPlayer _asthird_person_character)
  (Variables|Default|SetBlockable true))

(event Collision|EventActorEndOverlap
  (params (OtherActor :type Actor%20Object%20Reference))
  (Variables|Default|SetBlockable false))

(fn ConstructionScript)

(fn FindPlayerTarget
  (bind _outactors (Actor|GetAllActorsOfClass "/Game/ThirdPersonBP/Blueprints/ThirdPersonCharacter.ThirdPersonCharacter_C"))
  (for _array_element _outactors
    (if (< (Math|Vector|VectorLength (- (Transformation|GetActorLocation) (Transformation|GetWorldLocation (Variables|/Script/Engine.Character|GetMesh _array_element)))) (LocalVariables|GetClosestDistance))
      (LocalVariables|SetClosestDistance (Math|Vector|VectorLength (- (Transformation|GetActorLocation) (Transformation|GetWorldLocation (Variables|/Script/Engine.Character|GetMesh _array_element)))))
      (LocalVariables|SetClosestTarget _array_element)))
  (return (Variables|/Script/Engine.Character|GetMesh _array_element)))